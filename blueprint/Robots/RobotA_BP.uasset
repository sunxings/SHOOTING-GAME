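; RobotA_BP is a suicide-bomber enemy robot that explodes on death or shortly after the player touches it.
; Incoming damage, scaled by a coefficient, drains health until it self-destructs.
; Capsule overlap with the player fires once, playing a warning sound and flashing light before the delayed blast.
; The explosion deals radial damage sparing other RobotA instances, adds force and a decal; two functions switch walk speed for undetected and detected states.
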(event `self.ReceiveAnyDamage`
  (params (Damage :type "Float (single-precision)") (DamageType :type "DamageType Object Reference") (InstigatedBy :type "Controller Object Reference") (DamageCauser :type "Actor Object Reference"))
  (bind _output_get (set `self.血量` (- (`self.血量`) (* Damage (`self.伤害系数`)))))
  (if (<= _output_get 0.0)
    (`self.自爆`)))

(event `自爆`
  (bind _returnvalue (`self.K2_GetActorLocation` self))
  (`GameplayStatics.SpawnEmitterAtLocation` "/Game/MilitaryWeapSilver/FX/P_Grenade_Explosion_01.P_Grenade_Explosion_01" _returnvalue (struct) (1.3 1.3 1.3))
  (`GameplayStatics.SpawnSoundAtLocation` "/Game/MilitaryWeapSilver/Sound/RocketLauncher/Cues/RocketLauncher_Explosion_Cue.RocketLauncher_Explosion_Cue" _returnvalue (struct) 1.0 1.0 0.0 null null)
  (bind _outactors (`GameplayStatics.GetAllActorsOfClass` "RobotA_BP_C"))
  (`GameplayStatics.ApplyRadialDamage` 100.0 (`self.K2_GetActorLocation`) 700.0 "/Script/Engine.DamageType" _outactors self (`AIBlueprintHelperLibrary.GetAIController` null))
  (`RadialForceComponent.FireImpulse` (`self.RadialForce`))
  (`GameplayStatics.SpawnDecalAtLocation` "/Game/材质/UWC_Bullet_Holes/Materials/M_Master_Normal_Texture.M_Master_Normal_Texture" (500.0 500.0 500.0) (`self.K2_GetActorLocation`) (struct :`Pitch` -90.0) 15.0)
  (`self.K2_DestroyActor`))

(event `self.Capsule.OnComponentBeginOverlap`
  (params (OverlappedComponent :type "PrimitiveComponent Object Reference") (OtherActor :type "Actor Object Reference") (OtherComp :type "PrimitiveComponent Object Reference") (OtherBodyIndex :type Integer) (bFromSweep :type Boolean) (SweepResult :type "HitResult Structure (by ref)"))
  (cast `/Game/蓝图/主角/主角_bp` OtherActor)
  (`/Engine/EditorBlueprintResources/StandardMacros.DoOnce` false
    (:`Completed`
      (`|ExecutionSequence`
        (:`then_0`
          (`GameplayStatics.SpawnSoundAtLocation` "/Game/MilitaryWeapSilver/Sound/GrenadeLauncher/Cues/GrenadeLauncher_Warning_Cue.GrenadeLauncher_Warning_Cue" (`self.K2_GetActorLocation`) (struct) 1.0 1.0 0.0 null null)
          (`KismetSystemLibrary.Delay` 1.3)
          (`self.自爆`))
        (:`then_1`
          (bind (_direction `_新建轨道_0`) (`Timeline|闪红光`)
            (:`Update`
              (`LightComponent.SetIntensity` (`self.PointLight`) (`KismetMathLibrary.Lerp` 0.0 10000.0 `_新建轨道_0`)))))))))

(fn `UserConstructionScript`)

(fn `发现之后`
  (set `CharacterMovementComponent.MaxWalkSpeed` 450.0 (`self.CharacterMovement`)))

(fn `没有发现`
  (set `CharacterMovementComponent.MaxWalkSpeed` 200.0 (`self.CharacterMovement`)))