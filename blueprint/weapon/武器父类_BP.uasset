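; Base weapon Blueprint that handles starting and stopping automatic fire for the player character.
; 开始射击 stores the character and, if ammo remains, sets its anim instance's firing flag and picks aimed or hip fire from the aiming flag.
; The chosen shot fires immediately, then repeats on a looping fire-rate timer until 结束射击 clears both timers and the flag.
; Aimed shot, hip shot and magazine swap are empty events, apparently left for child weapons.
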(event `结束射击`
  (set `/Game/蓝图/主角/主角_AniBP.射击？` false (`/Game/蓝图/主角/主角_bp.动画实例` (`self.主角`)))
  (`KismetSystemLibrary.K2_ClearAndInvalidateTimerHandle` (stale `开始射击` _returnvalue))
  (`KismetSystemLibrary.K2_ClearAndInvalidateTimerHandle` (stale `开始射击` _returnvalue_2)))

(event `瞄准射击`)

(event `开始射击`
  (params (`主角` :type "/Game/蓝图/主角/主角_bp Object Reference"))
  (bind (`_名字` `_弹夹数` `_类型` `_载弹量` `_射速`) (break `/Game/蓝图/武器/武器属性` (`self.武器属性`)))
  (bind _output_get (set `self.主角` `主角`))
  (if (not (<= (`self.剩余子弹`) 0))
    (bind `_动画实例` (`/Game/蓝图/主角/主角_bp.动画实例` _output_get))
    (set `/Game/蓝图/主角/主角_AniBP.射击？` true `_动画实例`)
    (if (`/Game/蓝图/主角/主角_AniBP.瞄准？` `_动画实例`)
      (`self.瞄准射击`)
      (bind _returnvalue (`KismetSystemLibrary.K2_SetTimerDelegate` (delegate `瞄准射击`) `_射速` true))
      (else
        (`self.腰射射击`)
        (bind _returnvalue_2 (`KismetSystemLibrary.K2_SetTimerDelegate` (delegate `腰射射击`) `_射速` true))))))

(event `切换弹夹`)

(event `腰射射击`)

(fn `UserConstructionScript`)