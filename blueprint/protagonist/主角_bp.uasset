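; Third-person protagonist character that moves, sprints, jumps, picks up a weapon, aims and shoots.
; A camera sphere trace stores the hit weapon and snaps it to a back socket; fire and reload are forwarded to it.
; A state enum gates actions, while AnimBP flags drive timed draw/holster and aiming, which slows movement, follows controller yaw and shortens the spring arm by timeline.
; Damage reduces health by a multiplier and prints it.
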(event `self.ReceiveBeginPlay`
  (bind `_as主角_ani_bp` (cast `/Game/蓝图/主角/主角_AniBP` (`SkeletalMeshComponent.GetAnimInstance` (`self.Mesh`))))
  (set `self.动画实例` `_as主角_ani_bp`))

(event `InputAxis|向前`
  (params (AxisValue :type "Float (single-precision)"))
  (bind (_returnvalue_roll _returnvalue_pitch _returnvalue_yaw) (`KismetMathLibrary.BreakRotator` (`self.GetControlRotation`)))
  (`self.AddMovementInput` (`KismetMathLibrary.GetForwardVector` (`KismetMathLibrary.MakeRotator` 0.0 0.0 _returnvalue_yaw)) AxisValue))

(event `InputAxis|向右`
  (params (AxisValue :type "Float (single-precision)"))
  (bind (_returnvalue_roll _returnvalue_pitch _returnvalue_yaw) (`KismetMathLibrary.BreakRotator` (`self.GetControlRotation`)))
  (`self.AddMovementInput` (`KismetMathLibrary.GetRightVector` (`KismetMathLibrary.MakeRotator` 0.0 0.0 _returnvalue_yaw)) AxisValue))

(event `InputAxis|鼠标x`
  (params (AxisValue :type "Float (single-precision)"))
  (`self.AddControllerYawInput` AxisValue))

(event `InputAxis|鼠标y`
  (params (AxisValue :type "Float (single-precision)"))
  (`self.AddControllerPitchInput` AxisValue))

(event `InputAction|冲刺`
  (params (Key :type "Key Structure"))
  (bind _charactermovement (`self.CharacterMovement`))
  (bind _returnvalue (`|EnumEquality` (`self.角色状态`) "NewEnumerator0"))
  (:`Pressed`
    (if _returnvalue
      (set `CharacterMovementComponent.MaxWalkSpeed` 700.0 _charactermovement)))
  (:`Released`
    (if _returnvalue
      (set `CharacterMovementComponent.MaxWalkSpeed` 300.0 _charactermovement))))

(event `InputAction|跳跃`
  (params (Key :type "Key Structure"))
  (:`Pressed`
    (`self.Jump`))
  (:`Released`
    (`self.StopJumping`)))

(event `InputAction|交互`
  (params (Key :type "Key Structure"))
  (bind _camera (`self.Camera`))
  (bind _returnvalue (`SceneComponent.K2_GetComponentLocation` _camera))
  (:`Pressed`
    (bind (_outhit _returnvalue_2) (`KismetSystemLibrary.SphereTraceSingle` :`Start` _returnvalue :`End` (+ _returnvalue (* (`SceneComponent.GetForwardVector` _camera) 450)) :`Radius` 10.0 :`TraceChannel` "TraceTypeQuery1" :`DrawDebugType` "ForDuration" :`DrawTime` 1.0))
    (if _returnvalue_2
      (bind `_as武器父类_bp` (cast `/Game/蓝图/武器/武器父类_BP` (`.HitActor` (`GameplayStatics.BreakHitResult` _outhit))))
      (set `self.武器实例` `_as武器父类_bp`)
      (`self.K2_AttachToComponent` `_as武器父类_bp` (`self.Mesh`) "背部插槽A" "SnapToTarget" "SnapToTarget" "SnapToTarget" true))))

(event `InputAction|切换武器`
  (params (Key :type "Key Structure"))
  (bind `_动画实例` (`self.动画实例`))
  (bind `_动画实例_2` (`self.动画实例`))
  (bind `_动画实例_3` (`self.动画实例`))
  (bind `_动画实例_4` (`self.动画实例`))
  (:`Pressed`
    (if (`|EnumEquality` (`self.角色状态`) "NewEnumerator0")
      (set `self.角色状态` "NewEnumerator2")
      (if (`/Game/蓝图/主角/主角_AniBP.持枪？` (`self.动画实例`))
        (set `/Game/蓝图/主角/主角_AniBP.存取武器` true `_动画实例_3`)
        (set `/Game/蓝图/主角/主角_AniBP.拿取武器方向` -1.0 `_动画实例_3`)
        (`KismetSystemLibrary.Delay` 0.1)
        (set `/Game/蓝图/主角/主角_AniBP.存取武器` false `_动画实例_4`)
        (set `/Game/蓝图/主角/主角_AniBP.持枪？` false `_动画实例_4`)
        (set `self.角色状态` "NewEnumerator0")
        (else
          (set `/Game/蓝图/主角/主角_AniBP.存取武器` true `_动画实例_2`)
          (set `/Game/蓝图/主角/主角_AniBP.拿取武器方向` 1.0 `_动画实例_2`)
          (`KismetSystemLibrary.Delay` 0.3)
          (set `/Game/蓝图/主角/主角_AniBP.存取武器` false `_动画实例`)
          (set `/Game/蓝图/主角/主角_AniBP.持枪？` true `_动画实例`)
          (set `self.角色状态` "NewEnumerator0"))))))

(event `InputAction|开枪`
  (params (Key :type "Key Structure"))
  (bind `_武器实例` (`self.武器实例`))
  (:`Pressed`
    (if (`/Game/蓝图/主角/主角_AniBP.持枪？` (`self.动画实例`))
      (`/Game/蓝图/武器/武器父类_BP.开始射击` `_武器实例` self)))
  (:`Released`
    (if (`/Game/蓝图/主角/主角_AniBP.持枪？` (`self.动画实例`))
      (`/Game/蓝图/武器/武器父类_BP.结束射击` `_武器实例`))))

(event `InputAction|换弹`
  (params (Key :type "Key Structure"))
  (:`Pressed`
    (if (`|EnumEquality` (`self.角色状态`) "NewEnumerator0")
      (`/Game/蓝图/武器/武器父类_BP.切换弹夹` (`self.武器实例`)))))

(event `InputAction|瞄准`
  (params (Key :type "Key Structure"))
  (:`Pressed`
    (if (and (`/Game/蓝图/主角/主角_AniBP.持枪？` (`self.动画实例`)) (`|EnumEquality` (`self.角色状态`) "NewEnumerator0"))
      (set `/Game/蓝图/主角/主角_AniBP.瞄准？` true (`self.动画实例`))
      (`self.瞄准状态`)
      (bind (_direction `_瞄准状态`) (`Timeline|瞄准` :!label _label)
        (:`Update`
          (set `SpringArmComponent.TargetArmLength` (`KismetMathLibrary.Lerp` 230.0 50.0 `_瞄准状态`) (`self.SpringArm`))))))
  (:`Released`
    (if (`/Game/蓝图/主角/主角_AniBP.持枪？` (`self.动画实例`))
      (set `/Game/蓝图/主角/主角_AniBP.瞄准？` false (`self.动画实例`))
      (`self.取消瞄准`)
      (goto _label :!via `Reverse`))))

(event `self.ReceiveAnyDamage`
  (params (Damage :type "Float (single-precision)") (DamageType :type "DamageType Object Reference") (InstigatedBy :type "Controller Object Reference") (DamageCauser :type "Actor Object Reference"))
  (bind _output_get (set `self.血量值` (- (`self.血量值`) (* Damage (`self.伤害系数`)))))
  (`KismetSystemLibrary.PrintString` (`KismetStringLibrary.Conv_DoubleToString` _output_get)))

(fn `UserConstructionScript`)

(fn `取消瞄准`
  (set `self.bUseControllerRotationYaw` false)
  (set `CharacterMovementComponent.bOrientRotationToMovement` true (`self.CharacterMovement`))
  (set `self.角色状态` "NewEnumerator0")
  (set `CharacterMovementComponent.MaxWalkSpeed` 300.0 (`self.CharacterMovement`)))

(fn `瞄准状态`
  (set `self.bUseControllerRotationYaw` true)
  (set `CharacterMovementComponent.bOrientRotationToMovement` false (`self.CharacterMovement`))
  (set `self.角色状态` "NewEnumerator1")
  (set `CharacterMovementComponent.MaxWalkSpeed` 180.0 (`self.CharacterMovement`)))